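; Character component that detects vaultable ledges, shows a prompt widget and moves the owner onto them.
; While not vaulting, Tick traces downward just ahead of the capsule, validating hit height, walkable slope and capsule clearance.
; A valid hit caches the end position and displays the widget.
; The vault tick lerps actor location without sweeping over VaultSpeed, used as a duration, then resets the state.
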(event EventTick
  (params (DeltaSeconds :type Float%20%28single-precision%29))
  (bind _vaultwidget (Variables|Default|GetVaultWidget))
  (Utilities|SwitchState
    (:NotVaulting
      (bind (_result _endinglocation) (CallFunction|CanVault))
      (if _result
        (Variables|Default|SetEndPosition _endinglocation)
        (if (not (UserInterface|Viewport|IsinViewport _vaultwidget))
          (UserInterface|Viewport|AddtoViewport _vaultwidget 0))
        (elif (UserInterface|Viewport|IsinViewport (Variables|Default|GetVaultWidget))
          (Widget|RemovefromParent (Variables|Default|GetVaultWidget)))))
    (:Vaulting
      (Class|VaultingComponent|VaultTick DeltaSeconds))))

(fn CanVault
  (if (Utilities|Enum|Equal(Enum) (Variables|Default|GetVaultState) "EVS_NotVault")
    (bind _output_get (LocalVariables|SetCapsule (Variables|/Script/Engine.Character|GetCapsuleComponent (Variables|Default|GetOwningCharacter))))
    (bind (_outhit _ishit) (CallFunction|TracetoVault _output_get))
    (if _ishit
      (bind (_result _endinglocation) (CallFunction|CavVaulttoHit (LocalVariables|GetCapsule) _outhit))
      (return _result _endinglocation)
      (else
        (return false "0, 0, 0")))
    (else
      (return false "0, 0, 0"))))

(fn TracetoVault
  (params (Capsule :type Capsule%20Component%20Object%20Reference))
  (bind _owningcharacter (Variables|Default|GetOwningCharacter))
  (bind _returnvalue (Transformation|GetActorLocation _owningcharacter))
  (bind _returnvalue_2 (Transformation|GetActorForwardVector _owningcharacter))
  (bind _returnvalue_3 (Components|Capsule|GetScaledCapsuleHalfHeight Capsule))
  (bind _returnvalue_4 (* _returnvalue_2 4e+01))
  (bind _returnvalue_5 (+ _returnvalue _returnvalue_4))
  (bind (_outhit _returnvalue_6) (Collision|LineTraceByChannel (+ _returnvalue_5 (Math|Vector|MakeVector 0.0 0.0 _returnvalue_3)) (- _returnvalue_5 (Math|Vector|MakeVector 0.0 0.0 _returnvalue_3)) "TraceTypeQuery1" false (Utilities|Array|MakeArray (Variables|Default|GetOwningCharacter)) "None"))
  (return _outhit _returnvalue_6))

(fn CavVaulttoHit
  (params (Capsule :type Capsule%20Component%20Object%20Reference) (HitResult :type Hit%20Result%20Structure))
  (bind (_bblockinghit _binitialoverlap _time _distance _location _impactpoint _normal _impactnormal _physmat _hitactor _hitcomponent _hitbonename _bonename _hititem _elementindex _faceindex _tracestart _traceend) (Collision|BreakHitResult HitResult))
  (bind _returnvalue (Components|Capsule|GetScaledCapsuleHalfHeight Capsule))
  (Utilities|FlowControl|Sequence
    (:then_0
      (if (not (Math|Float|InRange(Float) (- (.Z (Math|Vector|BreakVector _location)) (.Z (Math|Vector|BreakVector _traceend))) (Variables|Default|GetMinVaultingHeight) (Variables|Default|GetMaxVaultingHeight)))
        (return false "0, 0, 0")))
    (:then_1
      (if (< (.Z (Math|Vector|BreakVector (.Normal (Collision|BreakHitResult HitResult)))) (Class|CharacterMovementComponent|GetWalkableFloorZ (Variables|/Script/Engine.Character|GetCharacterMovement (Variables|Default|GetOwningCharacter))))
        (return false "0, 0, 0")))
    (:then_2
      (bind _output_get (LocalVariables|SetEndLoc (+ (.Location (Collision|BreakHitResult HitResult)) (Math|Vector|MakeVector 0.0 0.0 (Components|Capsule|GetScaledCapsuleHalfHeight Capsule)))))
      (bind _result (CallFunction|CheckCapsuleCollision (+ _output_get (Math|Vector|MakeVector 0.0 0.0 _returnvalue)) _returnvalue (Components|Capsule|GetScaledCapsuleRadius Capsule)))
      (if _result
        (return false "0, 0, 0")))
    (:then_3
      (return true (LocalVariables|GetEndLoc)))))

(fn CheckCapsuleCollision
  (params (Center :type Vector) (HalfHeight :type Float%20%28double-precision%29) (Radius :type Float%20%28double-precision%29))
  (bind _returnvalue (Collision|CapsuleOverlapActors Center Radius HalfHeight (Utilities|Array|MakeArray "ObjectTypeQuery1" "ObjectTypeQuery3" "ObjectTypeQuery4") "/Script/Engine.Actor"))
  (return _returnvalue))

(fn BPTickVault
  (params (DeltaSeconds :type Float%20%28double-precision%29))
  (Utilities|FlowControl|Sequence
    (:then_0
      (Variables|Default|SetProgress (Math|Float|Clamp(Float) (+ (Variables|Default|GetProgress) (/ DeltaSeconds (Variables|Default|GetVaultSpeed)))))
      (Transformation|SetActorLocation (Variables|Default|GetOwningCharacter) (Math|Vector|Lerp(Vector) (Variables|Default|GetStartingPosition) (Variables|Default|GetEndPosition) (Variables|Default|GetProgress)) false false))
    (:then_1
      (if (>= (Variables|Default|GetProgress) 1.0)
        (Variables|Default|SetVaultState "EVS_NotVault")))))